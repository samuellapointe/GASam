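; Fireball gameplay ability that launches a BP_Fireball projectile from the avatar pawn's eye point.
; Only the authority commits the ability and spawns the replicated projectile, with no client-side prediction, then ends it.
; The projectile follows view yaw and roll at a fixed upward pitch.
; It receives a GE_FireballDamage spec whose SetByCaller damage comes from a scalable float evaluated at ability level.
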(event `self.K2_ActivateAbility`
  (`self.K2_HasAuthority` ; Only the server can spawn actors that get \nreplicated. In a more involved implementation,\nwe would likely spawn a fake projectile on the\nclient and have it lerp to the server's version \nthen disappear. For this simple project, we'll\njust accept visible latency for the client.
    (:`True`
      (bind _returnvalue (`self.K2_CommitAbility`))
      (if _returnvalue
        (`self.SpawnProjectile`)
        (`self.K2_EndAbility`)
        (else
          (`self.K2_EndAbility`))))
    (:`False`
      (`self.K2_EndAbility`))))

(event `self.K2_OnEndAbility`
  (params (bWasCancelled :type Boolean)))

(fn `PrepareDamageEffect`
  (returns (ReturnValue :type "GameplayEffectSpecHandle Structure"))
  (bind _returnvalue (`KismetMathLibrary.Conv_IntToDouble` (`self.GetAbilityLevel`)))
  (bind _returnvalue_2 (`AbilitySystemBlueprintLibrary.AssignTagSetByCallerMagnitude` (`self.MakeOutgoingGameplayEffectSpec` "/Game/GAS/Effects/GE_FireballDamage.GE_FireballDamage_C" _returnvalue) (struct :`TagName` "GASam.Damage") (`AbilitySystemBlueprintLibrary.Conv_ScalableFloatToFloat` (`self.AbilityDamage`) _returnvalue)))
  (return _returnvalue_2))

(fn `SpawnProjectile`
  (bind _aspawn (cast `Pawn` (`self.GetAvatarActorFromActorInfo`)))
  (bind _returnvalue (`self.PrepareDamageEffect`))
  (bind (_outlocation _outrotation) (`Actor.GetActorEyesViewPoint` _aspawn))
  (`|SpawnActorFromClass` "/Game/Blueprints/Objects/BP_Fireball.BP_Fireball_C" (`KismetMathLibrary.MakeTransform` _outlocation (`KismetMathLibrary.MakeRotator` (.roll _outrotation) 15.0 (.yaw _outrotation))) "Undefined" "MultiplyWithRoot" null _returnvalue _aspawn))