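; GAS player character Blueprint that adds a debug damage key and a procedural death animation.
; Pressing V applies an instant damage GameplayEffect to the character's own Ability System Component.
; PlayDeathAnimation disables input and runs a timeline that feeds pitch and height to a multicast event moving the Cube.
; When the timeline finishes, it sends a Death.AnimationComplete gameplay event to itself.
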(event Custom|PlayDeathAnimation
  (Input|DisableInput 0)
  (bind (_direction _pitch _height) (Timeline|Timeline PlayFromStart)
    (:Update
      (CallFunction|MulticastUpdateDeathAnim _pitch _height))
    (:Finished
      (Ability|SendGameplayEventtoActor self "(TagName=\"GASam.GameplayEvent.Death.AnimationComplete\")"))))

(event Custom|DebugDamageEvent
  (GameplayEffects|ApplyGameplayEffectToSelf :self (Ability|GetAbilitySystemComponent 0) :GameplayEffectClass "/Game/GAS/Effects/GE_DebugInstantDamage.GE_DebugInstantDamage_C"))

(event Custom|MulticastUpdateDeathAnim
  (params (NewPitch :type Float%20%28double-precision%29) (NewZ :type Float%20%28double-precision%29))
  (Transformation|SetRelativeRotation (Variables|Default|GetCube) (Math|Rotator|MakeRotator 0.0 NewPitch 0.0) false false)
  (Transformation|SetRelativeLocation (Variables|Default|GetCube) (Math|Vector|MakeVector 0.0 0.0 NewZ) false false))

(event EventBeginPlay)

(event Collision|EventActorBeginOverlap
  (params (OtherActor :type Actor%20Object%20Reference)))

(event EventTick
  (params (DeltaSeconds :type Float%20%28single-precision%29)))

(event Input|KeyboardEvents|DebugKeyV
  (params (Key :type Key%20Structure :default "None") (ActionValue :type Input%20Action%20Value%20Structure))
  (:Pressed
    (CallFunction|DebugDamageEvent)))

(fn ConstructionScript)