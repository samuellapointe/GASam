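; BP_Fireball is a replicated projectile that explodes on overlapping any actor except its instigator, or expires after a fixed lifespan.
; On a hit it spawns the explosion FX and applies its damage GameplayEffect spec to the target's AbilitySystemComponent.
; Only the authority destroys it on a hit.
; Clients play the FX on Destroyed if replicated destruction beat their local overlap.
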(event `self.ReceiveBeginPlay`
  (`self.SetLifeSpan` 10.0) ; Auto destroy if it took too long to hit something
)

(event `self.Collider.OnComponentBeginOverlap`
  (params (OverlappedComponent :type "PrimitiveComponent Object Reference") (OtherActor :type "Actor Object Reference") (OtherComp :type "PrimitiveComponent Object Reference") (OtherBodyIndex :type Integer) (bFromSweep :type Boolean) (SweepResult :type "HitResult Structure (by ref)"))
  (`self.OnHitActor` OtherActor))

(event `self.ReceiveDestroyed`
  ; Handle case where the replication of the projectile unspawning takes place before the destruction FX could be played on the client.
  (`/Engine/EditorBlueprintResources/ActorMacros.Switch Has Authority`
    (:`Remote`
      (if (not (`self.bExplosionFXPlayed`))
        (`self.PlayExplosionFX`)))))

(fn `ApplyDamage`
  (params (HitActor :type "Actor Object Reference"))
  (bind _returnvalue (`AbilitySystemBlueprintLibrary.GetAbilitySystemComponent` HitActor))
  (`/Engine/EditorBlueprintResources/StandardMacros.IsValid` _returnvalue
    (:`Is Valid`
      (`AbilitySystemComponent.BP_ApplyGameplayEffectSpecToSelf` _returnvalue (`self.DamageEffectSpecHandle`)))))

(fn `OnHitActor`
  (params (HitActor :type "Actor Object Reference"))
  (if (== HitActor (`self.GetInstigator`))
    (return) ; Ignore collisions with the caster
    (else
      (`self.PlayExplosionFX`)
      (`self.ApplyDamage` HitActor)
      (`/Engine/EditorBlueprintResources/ActorMacros.Switch Has Authority`
        (:`Authority`
          (`self.K2_DestroyActor`))))))

(fn `PlayExplosionFX`
  (set `self.bExplosionFXPlayed` true)
  (`NiagaraFunctionLibrary.SpawnSystemAtLocation` "/Game/Assets/FX/FX_Explosion.FX_Explosion" (`self.K2_GetActorLocation`)))

(fn `UserConstructionScript`)